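; BP_MainActor is a player-controlled Blueprint that lets a key press request an actor spawn from the game mode.
; BeginPlay adds the IMC_ButtonToSpawn Enhanced Input mapping context and caches the BP_GameMode reference.
; A raw K key event prints a debug message and calls SpawnActor on that game mode.
; The IA_SpawnActor input action event is present but has no logic attached.
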(event `EnhancedInput|/Game/Blueprints/IA_SpawnActor`
  (params (ActionValue :type Boolean) (ElapsedSeconds :type "Float (double-precision)") (TriggeredSeconds :type "Float (double-precision)") (InputAction :type "InputAction Object Reference" :default "/Game/Blueprints/IA_SpawnActor.IA_SpawnActor"))
  ;[1 1 1] InputAction(R) or K on Keyboard
)

(event `Key|K`
  (params (Key :type "Key Structure"))
  ;[1 1 1] InputAction(R) or K on Keyboard
  (:`Pressed`
    (`KismetSystemLibrary.PrintString` "SpawnedSphere")
    (`/Game/Blueprints/BP_GameMode.Spawn Actor` (`self.GameMode`))))

(event `self.ReceiveBeginPlay`
  (bind _asplayer_controller (cast `PlayerController` (`self.GetController`)))
  (`EnhancedInputSubsystemInterface.AddMappingContext` (pcsubsystem `EnhancedInputLocalPlayerSubsystem` _asplayer_controller) "/Game/Blueprints/IMC_ButtonToSpawn.IMC_ButtonToSpawn" 0 (struct))
  (bind _asbp_game_mode (cast `/Game/Blueprints/BP_GameMode` (`GameplayStatics.GetGameMode`)))
  (set `self.GameMode` _asbp_game_mode))

(fn `UserConstructionScript`)