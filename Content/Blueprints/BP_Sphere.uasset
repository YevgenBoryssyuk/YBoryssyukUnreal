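; BP_Sphere is an actor that moves its Sphere component from a start point to an end point.
; On BeginPlay it caches the locations of the TargetPointStartLocation and TargetPointEndLocation actors found by class, then plays a Timeline.
; Each Timeline update lerps between the two locations and applies the result as the Sphere's relative location, without sweeping, although both inputs are world-space positions.
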(event `self.ReceiveBeginPlay`
  (`|ExecutionSequence`
    (:`then_0`
      ;[1 1 1] Рух від точки A до точки B, за допоомгою Targetpoints
      (bind _returnvalue (`GameplayStatics.GetActorOfClass` "/Game/Blueprints/TargetPointStartLocation.TargetPointStartLocation_C"))
      (set `self.StartLocation` (`self.K2_GetActorLocation` _returnvalue))
      (bind _returnvalue_2 (`GameplayStatics.GetActorOfClass` "/Game/Blueprints/TargetPointEndLocation.TargetPointEndLocation_C"))
      (set `self.EndLocation` (`self.K2_GetActorLocation` _returnvalue_2)))
    (:`then_1`
      (bind (_direction _newtrack_0) (`Timeline|Timeline`)
        (:`Update`
          (`SceneComponent.K2_SetRelativeLocation` (`self.Sphere`) (`KismetMathLibrary.VLerp` (`self.StartLocation`) (`self.EndLocation`) _newtrack_0) false false))))))

(fn `UserConstructionScript`)